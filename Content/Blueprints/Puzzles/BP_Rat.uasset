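; BP_Rat is a puzzle rat that kills the player on sphere overlap whenever its Cheese flag is false.
; On that overlap it turns toward the third-person character, plays a jump attack animation and calls Death on the character.
; GetCheese plays the same animation and a 2D sound, clears Cheese, and slides the skeletal mesh to a target relative location.
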(event `GetCheese`
  (`SkeletalMeshComponent.PlayAnimation` (`self.SkeletalMesh`) "/Game/Blueprints/rat_jump_Anim_Armature_Armature_Armature_Attack.rat_jump_Anim_Armature_Armature_Armature_Attack" false)
  (set `self.Cheese` false)
  (`GameplayStatics.PlaySound2D` "/Game/Audio/FarePeynireUlastiginda.FarePeynireUlastiginda" 1.0 1.0 0.0 null null)
  (`KismetSystemLibrary.MoveComponentTo` (`self.SkeletalMesh`) (`self.Target Relative Location`) (struct) false false 0.5))

(event `self.Sphere.OnComponentBeginOverlap`
  (params (OverlappedComponent :type "PrimitiveComponent Object Reference") (OtherActor :type "Actor Object Reference") (OtherComp :type "PrimitiveComponent Object Reference") (OtherBodyIndex :type Integer) (bFromSweep :type Boolean) (SweepResult :type "HitResult Structure (by ref)"))
  (if (`self.ActorHasTag` OtherActor "Player")
    (if (not (`self.Cheese`))
      (bind _asbp_third_person_character (cast `/Game/Blueprints/Player/BP_ThirdPersonCharacter` (`GameplayStatics.GetPlayerCharacter` 0)))
      (`self.K2_SetActorRotation` (`KismetMathLibrary.FindLookAtRotation` (`self.K2_GetActorLocation`) (`self.K2_GetActorLocation` _asbp_third_person_character)))
      (`SkeletalMeshComponent.PlayAnimation` (`self.SkeletalMesh`) "/Game/Blueprints/rat_jump_Anim_Armature_Armature_Armature_Attack.rat_jump_Anim_Armature_Armature_Armature_Attack" false)
      (`/Game/Blueprints/Player/BP_ThirdPersonCharacter.Death` _asbp_third_person_character))))

(fn `UserConstructionScript`)