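; BP_Aquarium is an aquarium puzzle actor whose ground responds to the player character's size form and which contains a death trigger.
; On BeginPlay it caches the third-person character and binds to its FormChange event.
; The big form disables Ground collision, while the other form sets it to query-only.
; Overlapping DeathTrigger with a Player-tagged actor plays a 2D sound and calls the player's Death.
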(event `self.ReceiveBeginPlay`
  (bind _asbp_third_person_character (cast `/Game/Blueprints/Player/BP_ThirdPersonCharacter` (`GameplayStatics.GetPlayerCharacter` 0)))
  (bind _output_get (set `self.Player` _asbp_third_person_character))
  (add `/Game/Blueprints/Player/BP_ThirdPersonCharacter.FormChange` _output_get (delegate `FormChange_Event`)))

(event `FormChange_Event`
  (params (IsBig :type Boolean))
  (`PrimitiveComponent.SetCollisionEnabled` (`self.Ground`) (select `bool` IsBig :`false` "QueryOnly" :`true` "NoCollision" :!type "ECollisionEnabled Enum")))

(event `self.DeathTrigger.OnComponentBeginOverlap`
  (params (OverlappedComponent :type "PrimitiveComponent Object Reference") (OtherActor :type "Actor Object Reference") (OtherComp :type "PrimitiveComponent Object Reference") (OtherBodyIndex :type Integer) (bFromSweep :type Boolean) (SweepResult :type "HitResult Structure (by ref)"))
  (if (`self.ActorHasTag` OtherActor "Player")
    (`GameplayStatics.SpawnSound2D` "/Game/Audio/SuyaDusus.SuyaDusus" 1.0 1.0 0.0 null)
    (`/Game/Blueprints/Player/BP_ThirdPersonCharacter.Death` (`self.Player`))))

(fn `UserConstructionScript`)