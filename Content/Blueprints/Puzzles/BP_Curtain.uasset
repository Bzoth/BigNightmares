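; Puzzle curtain that the player opens by grabbing a rope, with the player's size tied to whether it is open.
; Overlapping the rope grip runs a timeline that slides rope and curtains, carries the player on the grip socket with a looping animation, then makes them big.
; An interact event reverses the motion and shrinks the player.
; While open, a box trigger toggles size on enter and exit; the construction script can start it open.
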(event `self.ReceiveBeginPlay`
  (bind _asbp_third_person_character (cast `/Game/Blueprints/Player/BP_ThirdPersonCharacter` (`GameplayStatics.GetPlayerCharacter` 0)))
  (set `self.Player` _asbp_third_person_character))

(event `self.RopeGrip.OnComponentBeginOverlap`
  (params (OverlappedComponent :type "PrimitiveComponent Object Reference") (OtherActor :type "Actor Object Reference") (OtherComp :type "PrimitiveComponent Object Reference") (OtherBodyIndex :type Integer) (bFromSweep :type Boolean) (SweepResult :type "HitResult Structure (by ref)"))
  (bind _mesh (`Character.Mesh` (`self.Player`)))
  (if (`self.Down`)
    _
    (elif (`self.CanMove`)
      (set `self.CanMove` false)
      (`|ExecutionSequence`
        (:`then_0`
          (bind (_direction _rope _leftcurtain _rightcurtain) (`Timeline|RopeMove` :!via `PlayFromStart`)
            (:`Update`
              (`SceneComponent.K2_SetRelativeLocation` (`self.Rope`) (`KismetMathLibrary.MakeVector` -270.0 110.0 _rope) false false)
              (`SceneComponent.K2_SetRelativeLocation` (`self.L_Curtain`) (`KismetMathLibrary.MakeVector` _leftcurtain 60.0) false false)
              (`SceneComponent.K2_SetRelativeLocation` (`self.R_Curtain`) (`KismetMathLibrary.MakeVector` _rightcurtain 60.0) false false)
              (bind _player (`self.Player`)
                (:`then`
                  (`self.K2_SetActorLocation` _player (`SceneComponent.GetSocketLocation` (`self.Rope`) "Grip") false false))
                (:`else`)))
            (:`Finished`
              (`SkeletalMeshComponent.SetAnimationMode` (`Character.Mesh` (`self.Player`)) "AnimationBlueprint" true)
              (`/Game/Blueprints/Player/BP_ThirdPersonCharacter.MakeBig` (`self.Player`))
              (set `self.Down` true)
              (set `self.CanMove` true))))
        (:`then_1`
          (`SkeletalMeshComponent.SetAnimationMode` _mesh "AnimationBlueprint" true)
          (`SkeletalMeshComponent.PlayAnimation` _mesh "/Game/Assets/Character/Animations/AS_Rope.AS_Rope" true))
        (:`then_2`
          (`GameplayStatics.SpawnSound2D` "/Game/Audio/Curtain_Open.Curtain_Open" 1.0 1.0 0.0 null))))))

(event `self.Box.OnComponentBeginOverlap`
  (params (OverlappedComponent :type "PrimitiveComponent Object Reference") (OtherActor :type "Actor Object Reference") (OtherComp :type "PrimitiveComponent Object Reference") (OtherBodyIndex :type Integer) (bFromSweep :type Boolean) (SweepResult :type "HitResult Structure (by ref)"))
  (if (`self.ActorHasTag` OtherActor "Player")
    (if (`self.Down`)
      (if (not (`/Game/Blueprints/Player/BP_ThirdPersonCharacter.IsBig` (`self.Player`)))
        (`/Game/Blueprints/Player/BP_ThirdPersonCharacter.MakeBig` (`self.Player`))))))

(event `self.Box.OnComponentEndOverlap`
  (params (OverlappedComponent :type "PrimitiveComponent Object Reference") (OtherActor :type "Actor Object Reference") (OtherComp :type "PrimitiveComponent Object Reference") (OtherBodyIndex :type Integer))
  (if (`self.ActorHasTag` OtherActor "Player")
    (if (`self.Down`)
      (if (`/Game/Blueprints/Player/BP_ThirdPersonCharacter.IsBig` (`self.Player`))
        (`/Game/Blueprints/Player/BP_ThirdPersonCharacter.MakeSmall` (`self.Player`))))))

(event `/Game/Blueprints/Player/BPI_Interract.Interract`
  (if (`self.CanMove`)
    (if (`self.Down`)
      (`GameplayStatics.PlaySound2D` "/Game/Audio/Curtain_Close.Curtain_Close" 1.0 1.0 0.0 null null)
      (bind (_direction _rope _leftcurtain _rightcurtain) (`Timeline|Timeline` :!via `ReverseFromEnd`)
        (:`Update`
          (`SceneComponent.K2_SetRelativeLocation` (`self.Rope`) (`KismetMathLibrary.MakeVector` -270.0 110.0 _rope) false false)
          (`SceneComponent.K2_SetRelativeLocation` (`self.L_Curtain`) (`KismetMathLibrary.MakeVector` _leftcurtain 60.0) false false)
          (`SceneComponent.K2_SetRelativeLocation` (`self.R_Curtain`) (`KismetMathLibrary.MakeVector` _rightcurtain 60.0) false false))
        (:`Finished`
          (set `self.Down` false)
          (set `self.CanMove` true)
          (`/Game/Blueprints/Player/BP_ThirdPersonCharacter.MakeSmall` (`self.Player`)))))))

(fn `UserConstructionScript`
  (if (not (`self.StartsClosed`))
    (`SceneComponent.K2_SetRelativeLocation` (`self.Rope`) (-270.0 110.0 -190.0) false false)
    (`SceneComponent.K2_SetRelativeLocation` (`self.L_Curtain`) (-180.0 60.0 0.0) false false)
    (`SceneComponent.K2_SetRelativeLocation` (`self.R_Curtain`) (180.0 60.0 0.0) false false)
    (set `self.Down` true)
    (set `self.CanMove` true)))