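; BP_Scale is a puzzle balance scale that tips while a big player stands on its holder and reverses when the player leaves.
; A timeline rotates the bone and re-snaps the left and right pans to its sockets, with a sound on each change.
; The first timeline finish makes the rat get the cheese, then after a delay a fast looping timer pins the rat to an offset from a cube.
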(event `asdasdasd`
  (`self.K2_SetActorLocation` (`self.rat`) (- (`SceneComponent.K2_GetComponentLocation` (`self.Cube`)) (0.0 160.0 0.0)) false false))

(event `self.ReceiveBeginPlay`
  (bind _bone (`self.Bone`))
  (`|ExecutionSequence`
    (:`then_0`
      (bind _asbp_third_person_character (cast `/Game/Blueprints/Player/BP_ThirdPersonCharacter` (`GameplayStatics.GetPlayerCharacter` 0)))
      (set `self.Player` _asbp_third_person_character))
    (:`then_1`
      (`SceneComponent.K2_SetWorldLocation` (`self.Left`) (`SceneComponent.GetSocketLocation` _bone "Left") false false :!label _label)
      (`SceneComponent.K2_SetWorldLocation` (`self.Right`) (`SceneComponent.GetSocketLocation` _bone "Right") false false))))

(event `self.ScaleHolder.OnComponentBeginOverlap`
  (params (OverlappedComponent :type "PrimitiveComponent Object Reference") (OtherActor :type "Actor Object Reference") (OtherComp :type "PrimitiveComponent Object Reference") (OtherBodyIndex :type Integer) (bFromSweep :type Boolean) (SweepResult :type "HitResult Structure (by ref)"))
  (if (`self.ActorHasTag` OtherActor "Player")
    (if (`/Game/Blueprints/Player/BP_ThirdPersonCharacter.IsBig` (`self.Player`))
      (`GameplayStatics.PlaySound2D` "/Game/Audio/Terazi.Terazi" 1.0 1.0 0.0 null null)
      (bind (_direction _bonerotation) (`Timeline|Scale` :!label _label_2)
        (:`Update`
          (`SceneComponent.K2_SetRelativeRotation` (`self.Bone`) (`KismetMathLibrary.MakeRotator` 0.0 _bonerotation) false false)
          (goto _label))
        (:`Finished`
          (`/Engine/EditorBlueprintResources/StandardMacros.DoOnce` false
            (:`Completed`
              (`/Game/Blueprints/Puzzles/BP_Rat.GetCheese` (`self.rat`))
              (`KismetSystemLibrary.Delay` 1.0)
              (`KismetSystemLibrary.K2_SetTimerDelegate` (delegate `asdasdasd`) 0.01 true))))))))

(event `self.ScaleHolder.OnComponentEndOverlap`
  (params (OverlappedComponent :type "PrimitiveComponent Object Reference") (OtherActor :type "Actor Object Reference") (OtherComp :type "PrimitiveComponent Object Reference") (OtherBodyIndex :type Integer))
  (if (`self.ActorHasTag` OtherActor "Player")
    (`GameplayStatics.PlaySound2D` "/Game/Audio/Terazi.Terazi" 1.0 1.0 0.0 null null)
    (goto _label_2 :!via `Reverse`)))

(fn `UserConstructionScript`)