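; Climbable ladder actor that attaches the player at the bottom and releases them at either end.
; The bottom trigger toggles CanClimb; Climb snaps the player to the Bottom point, starts a paused looping climb animation and enables the movement plane constraint.
; Reaching the bottom trigger restores the animation blueprint and free movement.
; The top trigger plays a climb-up montage, zeroing gravity until a notify places the player on top.
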(event `self.TopCol.OnComponentBeginOverlap`
  (params (OverlappedComponent :type "PrimitiveComponent Object Reference") (OtherActor :type "Actor Object Reference") (OtherComp :type "PrimitiveComponent Object Reference") (OtherBodyIndex :type Integer) (bFromSweep :type Boolean) (SweepResult :type "HitResult Structure (by ref)"))
  (bind _top (`self.Top`))
  (bind _top1 (`self.Top1`))
  (bind _charactermovement (`Character.CharacterMovement` (`self.Player`)))
  (bind _mesh (`Character.Mesh` (`self.Player`)))
  (if (and (`self.ActorHasTag` OtherActor "Player") (`/Game/Blueprints/Player/BP_ThirdPersonCharacter.Climbing` (`self.Player`)))
    (set `/Game/Blueprints/Player/BP_ThirdPersonCharacter.Climbing` false (`self.Player`))
    (set `SkeletalMeshComponent.bPauseAnims` false _mesh)
    (`SkeletalMeshComponent.SetAnimationMode` _mesh "AnimationBlueprint" true)
    (`|PlayMontage` _mesh "/Game/Assets/Character/CVlimbUpMontage.CVlimbUpMontage"
      (:`then`
        (set `CharacterMovementComponent.GravityScale` 0.0 (`Character.CharacterMovement` (`self.Player`)))
        (`self.K2_SetActorLocationAndRotation` (`self.Player`) (`SceneComponent.K2_GetComponentLocation` _top1) (`SceneComponent.K2_GetComponentRotation` _top1) false false))
      (:`OnNotifyBegin`
        (set `/Game/Blueprints/Player/BP_ThirdPersonCharacter.GoUp` true (`self.Player`))
        (`self.K2_SetActorLocationAndRotation` (`self.Player`) (`SceneComponent.K2_GetComponentLocation` _top) (`SceneComponent.K2_GetComponentRotation` _top) false false)
        (set `CharacterMovementComponent.GravityScale` 1.75 _charactermovement)
        (`MovementComponent.SetPlaneConstraintEnabled` _charactermovement false)))))

(event `self.Climb`
  (bind _player (`self.Player`))
  (bind _bottom (`self.Bottom`))
  (bind _mesh (`Character.Mesh` (`self.Player`)))
  (if (not (`/Game/Blueprints/Player/BP_ThirdPersonCharacter.Climbing` (`self.Player`)))
    (`SkeletalMeshComponent.SetAnimationMode` _mesh "AnimationSingleNode" true)
    (`SkeletalMeshComponent.PlayAnimation` _mesh "/Game/Assets/Character/Animations/AS_ClimbUp.AS_ClimbUp" true)
    (set `SkeletalMeshComponent.bPauseAnims` true _mesh)
    (`self.K2_SetActorLocationAndRotation` (`self.Player`) (`SceneComponent.K2_GetComponentLocation` _bottom) (`SceneComponent.K2_GetComponentRotation` _bottom) false false)
    (set `/Game/Blueprints/Player/BP_ThirdPersonCharacter.Climbing` true _player)
    (`MovementComponent.SetPlaneConstraintEnabled` (`Character.CharacterMovement` _player) true)))

(event `self.ReceiveBeginPlay`
  (bind _asbp_third_person_character (cast `/Game/Blueprints/Player/BP_ThirdPersonCharacter` (`GameplayStatics.GetPlayerCharacter` 0)))
  (set `self.Player` _asbp_third_person_character))

(event `self.BottomCol.OnComponentBeginOverlap`
  (params (OverlappedComponent :type "PrimitiveComponent Object Reference") (OtherActor :type "Actor Object Reference") (OtherComp :type "PrimitiveComponent Object Reference") (OtherBodyIndex :type Integer) (bFromSweep :type Boolean) (SweepResult :type "HitResult Structure (by ref)"))
  (bind _bottom1 (`self.Bottom1`))
  (bind _player (`self.Player`))
  (bind _mesh (`Character.Mesh` (`self.Player`)))
  (if (`self.ActorHasTag` OtherActor "Player")
    (set `/Game/Blueprints/Player/BP_ThirdPersonCharacter.CanClimb` true (`self.Player`))
    (bind _player_2 (`self.Player`)
      (:`then`
        (if (`/Game/Blueprints/Player/BP_ThirdPersonCharacter.Climbing` _player_2)
          (set `/Game/Blueprints/Player/BP_ThirdPersonCharacter.Climbing` false (`self.Player`))
          (set `SkeletalMeshComponent.bPauseAnims` false _mesh)
          (`SkeletalMeshComponent.SetAnimationMode` _mesh "AnimationBlueprint" true)
          (`self.K2_SetActorLocationAndRotation` (`self.Player`) (`SceneComponent.K2_GetComponentLocation` _bottom1) (`SceneComponent.K2_GetComponentRotation` _bottom1) false false)
          (set `/Game/Blueprints/Player/BP_ThirdPersonCharacter.GoUp` true _player)
          (`MovementComponent.SetPlaneConstraintEnabled` (`Character.CharacterMovement` _player) false)))
      (:`else`))))

(event `self.BottomCol.OnComponentEndOverlap`
  (params (OverlappedComponent :type "PrimitiveComponent Object Reference") (OtherActor :type "Actor Object Reference") (OtherComp :type "PrimitiveComponent Object Reference") (OtherBodyIndex :type Integer))
  (if (`self.ActorHasTag` OtherActor "Player")
    (set `/Game/Blueprints/Player/BP_ThirdPersonCharacter.CanClimb` false (`self.Player`))))

(fn `UserConstructionScript`)