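; BP_Puppet is a proximity hazard that kills the player for not sneaking while inside its sphere.
; Entering the sphere caches the player character and starts a looping one-second timer that polls its Sneak flag; leaving clears the timer.
; When a check finds the player not sneaking, it makes two child actor components visible, stops the timer, and calls the player's Death after a brief delay.
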(event `self.Sphere.OnComponentBeginOverlap`
  (params (OverlappedComponent :type "PrimitiveComponent Object Reference") (OtherActor :type "Actor Object Reference") (OtherComp :type "PrimitiveComponent Object Reference") (OtherBodyIndex :type Integer) (bFromSweep :type Boolean) (SweepResult :type "HitResult Structure (by ref)"))
  (if (`self.ActorHasTag` OtherActor "Player")
    (bind _asbp_third_person_character (cast `/Game/Blueprints/Player/BP_ThirdPersonCharacter` OtherActor))
    (set `self.Player` _asbp_third_person_character)
    (bind _returnvalue (`KismetSystemLibrary.K2_SetTimerDelegate` (delegate `Sneakwalk`) 1.0 true))
    (set `self.Puppet Timer` _returnvalue)))

(event `Sneakwalk`
  (if (not (`/Game/Blueprints/Player/BP_ThirdPersonCharacter.Sneak` (`self.Player`)))
    (`SceneComponent.SetVisibility` (`self.ChildActor`) true false)
    (`SceneComponent.SetVisibility` (`self.ChildActor1`) true false)
    (`KismetSystemLibrary.K2_ClearAndInvalidateTimerHandle` (`self.Puppet Timer`))
    (`KismetSystemLibrary.Delay` 0.5)
    (`/Game/Blueprints/Player/BP_ThirdPersonCharacter.Death` (`self.Player`))))

(event `self.Sphere.OnComponentEndOverlap`
  (params (OverlappedComponent :type "PrimitiveComponent Object Reference") (OtherActor :type "Actor Object Reference") (OtherComp :type "PrimitiveComponent Object Reference") (OtherBodyIndex :type Integer))
  (if (`self.ActorHasTag` OtherActor "Player")
    (`KismetSystemLibrary.K2_ClearAndInvalidateTimerHandle` (`self.Puppet Timer`))))

(fn `UserConstructionScript`)