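; BP_Cat is a sleeping-cat hazard that kills the player for not sneaking nearby.
; While the player overlaps its sphere, a looping one-second timer checks the character's Sneak flag, and leaving clears it.
; A failed check stops the timer, swaps the skeletal mesh to play the wake-up animation with a cat sound, then after a short delay fades the sound and calls Death on the player.
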(event `self.Sphere.OnComponentBeginOverlap`
  (params (OverlappedComponent :type "PrimitiveComponent Object Reference") (OtherActor :type "Actor Object Reference") (OtherComp :type "PrimitiveComponent Object Reference") (OtherBodyIndex :type Integer) (bFromSweep :type Boolean) (SweepResult :type "HitResult Structure (by ref)"))
  (if (`self.ActorHasTag` OtherActor "Player")
    (bind _asbp_third_person_character (cast `/Game/Blueprints/Player/BP_ThirdPersonCharacter` OtherActor))
    (set `self.Player` _asbp_third_person_character)
    (bind _returnvalue (`KismetSystemLibrary.K2_SetTimerDelegate` (delegate `Sneakwalk`) 1.0 true))
    (set `self.Cat Timer` _returnvalue)))

(event `Sneakwalk`
  (bind _skeletalmesh (`self.SkeletalMesh`))
  (if (not (`/Game/Blueprints/Player/BP_ThirdPersonCharacter.Sneak` (`self.Player`)))
    (`SkeletalMeshComponent.SetSkeletalMeshAsset` _skeletalmesh "/Game/Assets/cat_wakes_up_2.cat_wakes_up_2")
    (`SkeletalMeshComponent.PlayAnimation` _skeletalmesh "/Game/Assets/cat_wakes_up_2_Anim.cat_wakes_up_2_Anim" false)
    (`KismetSystemLibrary.K2_ClearAndInvalidateTimerHandle` (`self.Cat Timer`))
    (bind _returnvalue (`GameplayStatics.SpawnSound2D` "/Game/Audio/Cat.Cat" 1.0 1.0 0.0 null))
    (`KismetSystemLibrary.Delay` 1.0)
    (`AudioComponent.FadeOut` _returnvalue 1.0 0.0 "Linear")
    (`/Game/Blueprints/Player/BP_ThirdPersonCharacter.Death` (`self.Player`))))

(event `self.Sphere.OnComponentEndOverlap`
  (params (OverlappedComponent :type "PrimitiveComponent Object Reference") (OtherActor :type "Actor Object Reference") (OtherComp :type "PrimitiveComponent Object Reference") (OtherBodyIndex :type Integer))
  (if (`self.ActorHasTag` OtherActor "Player")
    (`KismetSystemLibrary.K2_ClearAndInvalidateTimerHandle` (`self.Cat Timer`))))

(fn `UserConstructionScript`)